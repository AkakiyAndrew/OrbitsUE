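; BP_OrbitalPawn is a player-controlled pawn that steers and thrusts through the Orbit world using direct key bindings.
; Each press of W adds a forward velocity kick, scaled by MaxThrust, to its OrbitDynamicObject.
; A and D step the yaw rate down or up, and Space zeroes all rotation.
; Tick runs the parent logic, then applies that persistent spin as a frame-rate-independent local rotation.
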(event `self.ReceiveTick`
  (params (DeltaSeconds :type "Float (single-precision)"))
  (`parent.ReceiveTick` DeltaSeconds)
  (`self.K2_AddActorLocalRotation` (* (`self.RotatingSpeed`) DeltaSeconds)))

(event `Key|W`
  (params (Key :type "Key Structure"))
  (:`Pressed`
    (`OrbitDynamicObjectComponent.AddVelocity` (`self.OrbitDynamicObject`) (* (`self.GetActorForwardVector`) (`self.MaxThrust`)))))

(event `Key|SpaceBar`
  (params (Key :type "Key Structure"))
  (:`Pressed`
    (set `self.RotatingSpeed` (struct))))

(event `Key|A`
  (params (Key :type "Key Structure"))
  (bind (_rotatingspeed_roll _rotatingspeed_pitch _rotatingspeed_yaw) (`KismetMathLibrary.BreakRotator` (`self.RotatingSpeed`)))
  (:`Pressed`
    (set `self.RotatingSpeed` (`KismetMathLibrary.MakeRotator` _rotatingspeed_roll _rotatingspeed_pitch (+ _rotatingspeed_yaw -5.0)))))

(event `Key|D`
  (params (Key :type "Key Structure"))
  (bind (_rotatingspeed_roll _rotatingspeed_pitch _rotatingspeed_yaw) (`KismetMathLibrary.BreakRotator` (`self.RotatingSpeed`)))
  (:`Pressed`
    (set `self.RotatingSpeed` (`KismetMathLibrary.MakeRotator` _rotatingspeed_roll _rotatingspeed_pitch (+ _rotatingspeed_yaw 5.0)))))

(event `Key|Q`
  (params (Key :type "Key Structure")))

(event `Key|E`
  (params (Key :type "Key Structure")))

(fn `UserConstructionScript`)