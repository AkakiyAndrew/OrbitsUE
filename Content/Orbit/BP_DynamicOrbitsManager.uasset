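; Manager actor that moves BP_OrbitDynamicObject actors under the Newtonian gravity of all BP_AttractorBase actors, both gathered at BeginPlay.
; Tick accumulates time-scaled delta and runs fixed-size substeps, always passing a current time of zero.
; Each Step applies a velocity-Verlet-style position and velocity update and draws a red debug motion line.
; ComputeAcceleration sums inverse-square pulls from each attractor's GM and mass center at a given time.
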(event `self.ReceiveBeginPlay`
  (`|ExecutionSequence`
    (:`then_0`
      (bind _outactors (`GameplayStatics.GetAllActorsOfClass` "/Game/Orbit/BP_AttractorBase.BP_AttractorBase_C"))
      (set `self.Attractors` _outactors))
    (:`then_1`
      (bind _outactors_2 (`GameplayStatics.GetAllActorsOfClass` "/Game/Orbit/BP_OrbitDynamicObject.BP_OrbitDynamicObject_C"))
      (set `self.Dynamic Objects` _outactors_2))))

(event `self.ReceiveTick`
  (params (DeltaSeconds :type "Float (single-precision)"))
  (bind _output_get (set `self.TimeAccumulator` (+ (* DeltaSeconds (`self.TimeScale `)) (`self.TimeAccumulator`))))
  (while (>= _output_get (`self.FixedStep `))
    (`|ExecutionSequence`
      (:`then_0`
        (`self.Step` (`self.FixedStep `)))
      (:`then_1`
        (set `self.TimeAccumulator` (- (`self.TimeAccumulator`) (`self.FixedStep `)))))))

(fn `ComputeAcceleration`
  (params (Position :type "Vector Structure") (Time :type "Float (double-precision)"))
  (returns (Acceleration :type "Vector Structure"))
  (locals (Accel :type "Vector Structure"))
  (`|ExecutionSequence`
    (:`then_0`
      (for _array_element (`self.Attractors`)
        (bind _returnvalue (- (`/Game/Orbit/BP_AttractorBase.GetMassCenterPosition` _array_element Time) Position))
        (bind _returnvalue_2 (`KismetMathLibrary.VSizeSquared` _returnvalue))
        (set `local.Accel` (+ (`local.Accel`) (* (* _returnvalue (`/Game/Orbit/BP_AttractorBase.GetBodyGM` _array_element)) (/ 1.0 (* (`KismetMathLibrary.Sqrt` _returnvalue_2) _returnvalue_2)))))))
    (:`then_1`
      (return (`local.Accel`)))))

(fn `Step`
  (params (TimeDelta :type "Float (double-precision)") (`Current Time` :type "Float (double-precision)"))
  (locals (NewPos :type "Vector Structure"))
  (for _array_element (`self.Dynamic Objects`)
    (bind _returnvalue (`self.K2_GetActorLocation` _array_element))
    (bind _acceleration (`self.ComputeAcceleration` _returnvalue `Current Time`))
    (bind _velocity (`/Game/Orbit/BP_OrbitDynamicObject.Velocity` _array_element))
    (bind _returnvalue_2 (+ (* (* _acceleration 0.5) (`KismetMathLibrary.MultiplyMultiply_FloatFloat` TimeDelta 2.0)) (+ _returnvalue (* _velocity TimeDelta))))
    (`self.K2_SetActorLocation` _array_element _returnvalue_2 false false)
    (set `/Game/Orbit/BP_OrbitDynamicObject.Velocity` (+ _velocity (* (* (+ _acceleration (`self.ComputeAcceleration` _returnvalue (+ `Current Time` TimeDelta))) 0.5) TimeDelta)) _array_element)
    (`KismetSystemLibrary.DrawDebugLine` _returnvalue (+ _returnvalue (* (- _returnvalue_2 _returnvalue) 100.0)) (struct :`R` 1.0 :`G` 0.011082 :`A` 1.0) 0.0 1.0)))

(fn `UserConstructionScript`)