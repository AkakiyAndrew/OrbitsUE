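; Orbiting object Blueprint that visualizes its predicted trajectory and exposes fixed velocity nudges along positive and negative X and Y.
; On each prediction update from the parent class, it pushes the predicted points and their count into a Niagara ribbon.
; Tick also draws debug spheres and lines along the prediction, marking the orbital position and last predicted point.
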(event `OnPredictionUpdate_Event`
  (bind _returnvalue (`self.GetPredictionPoints`))
  (bind _ns_ribbonlink (`self.NS_RibbonLink`))
  (`NiagaraComponent.SetVariableInt` _ns_ribbonlink "Points Count" (`KismetArrayLibrary.Array_Length` _returnvalue))
  (`NiagaraDataInterfaceArrayFunctionLibrary.SetNiagaraArrayPosition` _ns_ribbonlink "Position Array" _returnvalue))

(event `self.ReceiveBeginPlay`
  (add `self.OnPredictionUpdate` (delegate `OnPredictionUpdate_Event`)))

(event `self.ReceiveTick`
  (params (DeltaSeconds :type "Float (single-precision)"))
  (bind _returnvalue (`self.GetPredictionPoints`))
  (`parent.ReceiveTick` DeltaSeconds)
  (`|ExecutionSequence`
    (:`then_0`
      (for (_array_element _array_index) _returnvalue
        (`KismetSystemLibrary.DrawDebugSphere` _array_element 5.0 6 (struct :`R` 1.0 :`G` 1.0 :`B` 1.0 :`A` 1.0) 0.0 1.0 "Foreground")
        (bind _returnvalue_2 (- _array_index 1))
        (if (`KismetArrayLibrary.Array_IsValidIndex` _returnvalue _returnvalue_2)
          (`KismetSystemLibrary.DrawDebugLine` _array_element (`|GetArrayItem` _returnvalue _returnvalue_2) (struct :`R` 1.0 :`B` 0.724245 :`A` 1.0) 0.0 2.0 "Foreground"))))
    (:`then_1`
      (`KismetSystemLibrary.DrawDebugSphere` (`self.GetOrbitalPosition`) 100.0 12 (struct :`R` 1.0 :`G` 0.037271 :`B` 0.761 :`A` 1.0) 0.0 0.0 "Foreground")
      (`KismetSystemLibrary.DrawDebugSphere` (`self.GetLastPredictedPoint`) 100.0 12 (struct :`R` 1.0 :`G` 0.053468 :`B` 0.004753 :`A` 1.0) 0.0 0.0 "Foreground"))))

(fn `Add Neg To X`
  (`self.AddVelocity` (-10.0 0.0 0.0)))

(fn `Add Neg To Y`
  (`self.AddVelocity` (0.0 -10.0 0.0)))

(fn `Add Pos To X`
  (`self.AddVelocity` (10.0 0.0 0.0)))

(fn `Add Pos To Y`
  (`self.AddVelocity` (0.0 10.0 0.0)))

(fn `UserConstructionScript`)